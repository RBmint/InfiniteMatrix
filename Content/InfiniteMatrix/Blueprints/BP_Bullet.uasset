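; BP_Bullet is a projectile that moves along world X each tick by a swept offset scaled by ForwardSpeed.
; When its Sphere begins overlapping a BP_Tunnel, it destroys every BP_Bullet in the level, not just itself.
; If the sphere touches that tunnel's Enemy component, it also raises the BP_Player score, updates the score widget, and increases the player's forward speed at every fifth point.
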(event OnComponentBeginOverlap(Sphere)
  (params (OverlappedComponent :type Primitive%20Component%20Object%20Reference) (OtherActor :type Actor%20Object%20Reference) (OtherComp :type Primitive%20Component%20Object%20Reference) (OtherBodyIndex :type Integer) (bFromSweep :type Boolean) (SweepResult :type Hit%20Result%20Structure%20%28by%20ref%29))
  (bind _asbp_tunnel (Utilities|Casting|CastToBP_Tunnel OtherActor))
  (if (Class|PrimitiveComponent|IsOverlappingComponent (Variables|Default|GetSphere) (Variables|/Game/InfiniteMatrix/Blueprints/BP_Tunnel.BP_Tunnel_C|GetEnemy _asbp_tunnel))
    (bind _outactors (Actor|GetAllActorsOfClass "BP_Bullet_C"))
    (Actor|DestroyActor _outactors)
    (bind _asbp_player (Utilities|Casting|CastToBP_Player (Game|Player|GetPlayerPawn 0)))
    (bind _output_get (Variables|/Game/InfiniteMatrix/Blueprints/BP_Player.BP_Player_C|SetPlayerScore _asbp_player (+ (Variables|/Game/InfiniteMatrix/Blueprints/BP_Player.BP_Player_C|GetPlayerScore _asbp_player) 1)))
    (Default|UpdateScore (Variables|/Game/InfiniteMatrix/Blueprints/BP_Player.BP_Player_C|GetWB_Score _asbp_player) _output_get)
    ;[1 1 1] Add forward speed when score mod 5 = 0
    (if (== (Math|Integer|%(Integer) (Variables|/Game/InfiniteMatrix/Blueprints/BP_Player.BP_Player_C|GetPlayerScore _asbp_player) 5) 0)
      (Variables|/Game/InfiniteMatrix/Blueprints/BP_Player.BP_Player_C|SetForwardSpeed _asbp_player (+ (Variables|/Game/InfiniteMatrix/Blueprints/BP_Player.BP_Player_C|GetForwardSpeed _asbp_player) 2.5e+02)))
    (else
      (bind _outactors_2 (Actor|GetAllActorsOfClass "BP_Bullet_C"))
      (Actor|DestroyActor _outactors_2))))

(event EventBeginPlay)

(event Collision|EventActorBeginOverlap
  (params (OtherActor :type Actor%20Object%20Reference)))

(event EventTick
  (params (DeltaSeconds :type Float%20%28single-precision%29))
  ;[1 1 1] Set bullet speed
  (Transformation|AddActorWorldOffset (Math|Vector|MakeVector (.x (Math|Conversions|ToVector(Float) (* DeltaSeconds (Variables|Default|GetForwardSpeed)))) 0.0 0.0) true))

(fn ConstructionScript)